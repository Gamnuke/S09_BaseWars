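; Builder pawn that displays a tinted preview image of a part being placed.
; The construction script creates a dynamic material instance and applies it to both static and skeletal preview meshes.
; Tick eases the material's Intensity toward a resting value and colors it cyan when CanPlace is true, red otherwise.
; PostPlaceItem is empty; its apparent intensity flash and impact emitter logic is disconnected and never runs.
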(event `self.PostPlaceItem`
  (params (Part :type "Vector Structure")))

(event `self.ReceiveTick`
  (params (DeltaSeconds :type "Float (single-precision)"))
  (bind _mat (`self.Mat`))
  (bind _output_get (set `self.Intensity` (`KismetMathLibrary.FInterpTo` (`self.Intensity`) 0.5 DeltaSeconds 20.0)))
  (`MaterialInstanceDynamic.SetScalarParameterValue` (`self.Mat`) "Intensity" _output_get)
  (if (`self.CanPlace`)
    (`MaterialInstanceDynamic.SetVectorParameterValue` _mat "Color" (struct :`G` 1.0 :`B` 1.0 :`A` 1.0))
    (else
      (`MaterialInstanceDynamic.SetVectorParameterValue` _mat "Color" (struct :`R` 1.0 :`A` 1.0)))))

(fn `UserConstructionScript`
  (bind _returnvalue (`KismetMaterialLibrary.CreateDynamicMaterialInstance` "/Game/ImageMaterialInst.ImageMaterialInst" "Inst"))
  (bind _output_get (set `self.Mat` _returnvalue))
  (`PrimitiveComponent.SetMaterial` (`self.StaticPartImage`) 0 _output_get)
  (`PrimitiveComponent.SetMaterial` (`self.SkeletalPartImage`) 0 _output_get))