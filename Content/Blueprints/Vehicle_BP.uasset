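; Vehicle Blueprint whose construction script is empty, so it currently runs no logic of its own.
; An unconnected debug graph loops over mesh instances and their sockets, rotating and offsetting each socket by its instance's local-space transform.
; It would draw a short, thick colored line along each socket's combined up vector to visualize per-instance socket placement and orientation.
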(fn `UserConstructionScript`)