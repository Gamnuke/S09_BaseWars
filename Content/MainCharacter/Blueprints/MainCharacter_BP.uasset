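; Main player character with a zoomable boom camera that bobs to music bass.
; Tick turns BassAmplitude into a thresholded power curve that rises instantly and decays smoothly, scaling a fast vertical sine offset on the camera.
; The Zoom axis adjusts boom length within limits, and ServerLoadURL assigns a URL to a given Television.
; BeginPlay sets UI-only input and prints the remote network role for debugging.
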(event `self.ReceiveBeginPlay`
  (`WidgetBlueprintLibrary.SetInputMode_UIOnlyEx` (`GameplayStatics.GetPlayerController` 0) null)
  (`KismetSystemLibrary.PrintString` (`|GetEnumeratorNameAsString` (`self.GetRemoteRole`)) true true (struct :`R` 1.0 :`G` 0.262703 :`A` 1.0) 100.0))

(event `ServerLoadURL`
  (params (Television :type "/Game/Props/Television/Television Object Reference") (URL :type String))
  (set `/Game/Props/Television/Television.URL` URL Television))

(event `self.ReceiveTick`
  (params (DeltaSeconds :type "Float (single-precision)"))
  (bind _returnvalue (/ (`KismetMathLibrary.MultiplyMultiply_FloatFloat` (`KismetMathLibrary.FClamp` (- (`self.BassAmplitude`) 5.0) 0.0 100000.0) 1.55) 2.0))
  (if (> _returnvalue (`self.CurrentBass`))
    (set `self.CurrentBass` _returnvalue)
    (else
      (set `self.CurrentBass` (`KismetMathLibrary.FInterpTo` (`self.CurrentBass`) _returnvalue DeltaSeconds 8.0))))
  (`SceneComponent.K2_SetRelativeLocation` (`self.CameraComponent`) (`KismetMathLibrary.MakeVector` 0.0 60.0 (* (`KismetMathLibrary.Sin` (* (`GameplayStatics.GetTimeSeconds`) 50.0)) (`self.CurrentBass`))) false false))

(event `InputAxis|Zoom`
  (params (AxisValue :type "Float (single-precision)"))
  (bind _cameraboom (`self.CameraBoom`))
  (set `SpringArmComponent.TargetArmLength` (`KismetMathLibrary.FClamp` (+ (`SpringArmComponent.TargetArmLength` _cameraboom) (* AxisValue -10.0)) 0.0 300.0) _cameraboom))

(fn `UserConstructionScript`)